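; BP_Player is a player Blueprint that displays its own network roles through a widget, exposing local and remote role for inspection.
; On BeginPlay it casts the RoleWidget component's user widget to WBP_Role and sets its text from the enum names of the local and remote roles.
; The roles are read only once, and the construction script is empty.
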(event EventBeginPlay
  (bind _aswbp_role (Utilities|Casting|CastToWBP_Role (UserInterface|GetUserWidgetObject (Variables|Default|GetRoleWidget))))
  (Default|SetRemoteText _aswbp_role (Utilities|Text|ToText(String) (Utilities|String|EnumtoString (Class|Actor|GetRemoteRole))))
  (Default|SetLocalText _aswbp_role (Utilities|Text|ToText(String) (Utilities|String|EnumtoString (Networking|GetLocalRole)))))

(fn ConstructionScript)